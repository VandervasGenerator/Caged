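; Light switch Blueprint that turns a registered group of lights on and off together.
; ToggleLights alternates through a FlipFlop, setting every light's intensity to full or zero, tilting the switch mesh and playing a click sound at its location.
; RegisterLight adds lights to the Lights array, and RemoveEmptyLights removes an empty entry from it.
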(event `ToggleLights`
  (bind _isa (`/Engine/EditorBlueprintResources/StandardMacros.FlipFlop`)
    (:`A`
      _)
    (:`B`
      _))
  (for _array_element (`self.Lights`)
    (`LightComponent.SetIntensity` _array_element (* (`KismetMathLibrary.Conv_BoolToDouble` (not _isa)) 5000.0)))
  (`SceneComponent.K2_SetRelativeRotation` (`self.SwitchMesh`) (`KismetMathLibrary.MakeRotator` (select `bool` _isa :`true` 30.0 :!type "Float (single-precision)")) false true)
  (`GameplayStatics.PlaySoundAtLocation` "/Game/SoundFX/LightSwitch.LightSwitch" (`SceneComponent.K2_GetComponentLocation` (`self.SwitchMesh`))))

(event `RegisterLight`
  (params (`New Light` :type "LightComponent Object Reference"))
  (`KismetArrayLibrary.Array_Add` (`self.Lights`) `New Light`))

(event `RemoveEmptyLights`
  (`KismetArrayLibrary.Array_RemoveItem` (`self.Lights`)))

(fn `UserConstructionScript`)