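; Sculpture bust prop Blueprint that gives itself a random look.
; The construction script sets the Wig component to a random mesh from WigArray and randomly decides whether the Shades component gets the sunglasses mesh or none.
; It uses unseeded random nodes, so the look can change whenever construction reruns.
; The event graph holds only disabled placeholder events, so it has no gameplay logic.
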(fn `UserConstructionScript`
  (bind _wigarray (`self.WigArray`))
  (`StaticMeshComponent.SetStaticMesh` (`self.Wig`) (`|GetArrayItem` _wigarray (`KismetMathLibrary.RandomIntegerInRange` 0 (- (`KismetArrayLibrary.Array_Length` _wigarray) 1))))
  (`StaticMeshComponent.SetStaticMesh` (`self.Shades`) (select `bool` (`KismetMathLibrary.RandomBool`) :`true` "/Game/Caged/Geometry/Busts/CagedSculptureShades.CagedSculptureShades" :!type "StaticMesh Object Reference")))